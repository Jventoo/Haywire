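; AI controller for drones that runs the BT_Drone behavior tree and handles detection of the player.
; Perception updates start a detection timer scaled by distance, or detect instantly inside a set radius.
; Detection sets the intruder and line-of-sight blackboard keys and plays a robotic yell.
; Any other perception update cancels pending detection and starts a grace timer that clears those keys.
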(event `self.ReceivePossess`
  (params (PossessedPawn :type "Pawn Object Reference"))
  ;[1 1 1] Begin Possession
  (set `self.InitialLocation` (`self.K2_GetActorLocation` PossessedPawn))
  (`self.RunBehaviorTree` "/Game/Haywire/Blueprints/Drones/BT_Drone.BT_Drone"))

(event `PlayerFound`
  (bind _blackboard (`self.Blackboard`))
  ;[1 1 1] Update blackboard and begin chasing
  (`BlackboardComponent.SetValueAsBool` _blackboard (`self.HasLOS`) true)
  (`BlackboardComponent.SetValueAsObject` _blackboard (`self.Intruder`) (`self.IntruderActor`))
  (`GameplayStatics.SpawnSoundAttached` "/Game/Haywire/Audio/Effects/Drones/SC_RoboticYell.SC_RoboticYell" (`Actor.RootComponent` (`self.K2_GetPawn`)) "None" (0.0 0.0 0.0) (struct) "KeepRelativeOffset" false 1.0 1.0 0.0 null null))

(event `self.AIPerception.OnTargetPerceptionUpdated`
  (params (Actor :type "Actor Object Reference") (Stimulus :type "AIStimulus Structure"))
  (bind _returnvalue (`KismetMathLibrary.Vector_Distance` (`self.K2_GetActorLocation` Actor) (`self.K2_GetActorLocation` (`self.GetControlledDrone`))))
  ;[1 1 1] Check what our AI is sensing
  (set `self.IntruderActor` Actor)
  (if (and (`self.ActorHasTag` Actor "Player") (`.bSuccessfullySensed` (break `AIStimulus` Stimulus)))
    ;[1 1 1] Start counting down time until player is spotted at an interval determined by our distance, unless we are so close that it is instant
    (`KismetSystemLibrary.K2_ClearAndInvalidateTimerHandle` (`self.IntruderTimer`))
    (if (< _returnvalue (`self.InstantDetectionRadius`))
      (`self.PlayerFound`)
      (else
        (bind _output_get (set `self.DetectionTimer` (`KismetMathLibrary.MapRangeClamped` _returnvalue 400.0 1000.0 0.0 4.0)))
        (bind _returnvalue_2 (`KismetSystemLibrary.K2_SetTimerDelegate` (delegate `PlayerFound`) _output_get))
        (set `self.DetectionTimerHandle` _returnvalue_2)))
    (else
      ;[1 1 1] Decrement time until we consider the intruder as missing
      (`KismetSystemLibrary.K2_ClearAndInvalidateTimerHandle` (`self.DetectionTimerHandle`))
      (bind _returnvalue_3 (`KismetSystemLibrary.K2_SetTimerDelegate` (delegate `StartIntruderTimer`) (`self.LineOfSightTimer`)))
      (set `self.IntruderTimer` _returnvalue_3))))

(event `StartIntruderTimer`
  (bind _blackboard (`self.Blackboard`))
  ;[1 1 1] Decrement time until we consider the intruder as missing
  (`BlackboardComponent.SetValueAsBool` _blackboard (`self.HasLOS`) false)
  (`BlackboardComponent.SetValueAsObject` _blackboard (`self.Intruder`) null))

(fn `GetControlledDrone`
  (returns (Drone :type "/Game/Haywire/Blueprints/Drones/BP_DroneCharacter Object Reference"))
  (bind _asbp_drone_character (cast `/Game/Haywire/Blueprints/Drones/BP_DroneCharacter` (`self.K2_GetPawn`)))
  (return _asbp_drone_character))

(fn `UserConstructionScript`)