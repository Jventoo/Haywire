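; Enemy drone character in Haywire that can detect and kill the player, working alongside BP_DroneController.
; On spawn it sets its patrol location to a random point in the latter half of its PatrolPath spline.
; A detection sphere reports the player to the controller as an intruder, while a kill box kills a living player only during a chase.
; UpdateWalkSpeed exposes movement speed changes.
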(event `self.ReceiveBeginPlay`
  (bind _patrolpath (`self.PatrolPath`))
  (bind _returnvalue (`SplineComponent.GetNumberOfSplinePoints` _patrolpath))
  (set `self.PatrolLocation` (`SplineComponent.GetLocationAtSplinePoint` _patrolpath (`KismetMathLibrary.RandomIntegerInRange` (/ _returnvalue 2) (- _returnvalue 1)) "World")))

(event `self.InstantDetectionSphere.OnComponentBeginOverlap`
  (params (OverlappedComponent :type "PrimitiveComponent Object Reference") (OtherActor :type "Actor Object Reference") (OtherComp :type "PrimitiveComponent Object Reference") (OtherBodyIndex :type Integer) (bFromSweep :type Boolean) (SweepResult :type "HitResult Structure (by ref)"))
  (if (== OtherActor (`GameplayStatics.GetPlayerCharacter` 0))
    (bind _asbp_drone_controller (cast `/Game/Haywire/Blueprints/Drones/BP_DroneController` (`self.GetController`)))
    (set `/Game/Haywire/Blueprints/Drones/BP_DroneController.IntruderActor` OtherActor _asbp_drone_controller)
    (`/Game/Haywire/Blueprints/Drones/BP_DroneController.PlayerFound` _asbp_drone_controller)))

(event `self.KillBox.OnComponentBeginOverlap`
  (params (OverlappedComponent :type "PrimitiveComponent Object Reference") (OtherActor :type "Actor Object Reference") (OtherComp :type "PrimitiveComponent Object Reference") (OtherBodyIndex :type Integer) (bFromSweep :type Boolean) (SweepResult :type "HitResult Structure (by ref)"))
  (bind _returnvalue (`GameplayStatics.GetPlayerCharacter` 0))
  (if (== OtherActor _returnvalue)
    (bind _asbp_drone_controller (cast `/Game/Haywire/Blueprints/Drones/BP_DroneController` (`self.GetController`)))
    (bind _asbp_haywire_character (cast `/Game/Haywire/Blueprints/Player/BP_HaywireCharacter` _returnvalue))
    (if (and (`/Game/Haywire/Blueprints/Drones/BP_DroneController.bChasing` _asbp_drone_controller) (not (`/Game/Haywire/Blueprints/Player/BP_HaywireCharacter.bDead` _asbp_haywire_character)))
      (`/Game/Haywire/Blueprints/Player/BP_HaywireCharacter.KillPlayer` _asbp_haywire_character))))

(fn `UpdateWalkSpeed`
  (params (NewSpeed :type "Float (double-precision)"))
  (set `CharacterMovementComponent.MaxWalkSpeed` NewSpeed (`self.CharacterMovement`)))

(fn `UserConstructionScript`)