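; BP_Door is an interactable sliding door that can be locked behind a key ID, with material and light color showing its state.
; Interact checks the player controller for the key, then unlocks and opens with sound and steam, or shows a key message.
; A timeline lerps the panel; leaving the trigger reverses it.
; LockDoor applies the locked look and lowers an open door, but sets Locked to false.
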(event `LockDoor`
  (bind _unlockdoor (`self.UnlockDoor`))
  ;[1 1 1] Lock the door, update materials/sounds, and then bring it down if it was up
  (set `self.Locked` false)
  (`PrimitiveComponent.SetMaterial` (`self.Door_Small_UI`) 0 "/Game/ModSci_Engineer/Materials/UI/MI_Door_Locked.MI_Door_Locked")
  (`LightComponent.SetLightColor` (`self.PointLightb`) (`self.LockedLightColor`) true)
  (`LightComponent.SetLightColor` (`self.PointLight`) (`self.LockedLightColor`) true)
  (`AudioComponent.Play` _unlockdoor 0.0)
  (`KismetSystemLibrary.Delay` (+ (`SoundBase.Duration` (`AudioComponent.Sound` _unlockdoor)) 0.7))
  (if (not (`self.Interactable`))
    (bind (_direction _doorposition) (`Timeline|Timeline_0` :!via `Reverse` :!label _label)
      (:`Update`
        (`SceneComponent.K2_SetRelativeLocation` (`self.Door_Small_A`) (`KismetMathLibrary.VLerp` (`self.DoorClosed`) (`self.DoorOpen`) _doorposition) false false))
      (:`Finished`
        ;[1 1 1] If our door is back in its original position, we can now open it again
        (if (== (`SceneComponent.RelativeLocation` (`self.Door_Small_A`)) (`self.DoorClosed`))
          (set `self.Interactable` true))))))

(event `/Game/Haywire/Blueprints/Interactions/BPI_Interaction.Interact`
  (bind _unlockdoor (`self.UnlockDoor`))
  ;[1 1 1] Check to see if the door is locked
  (if (`self.Locked`)
    ;[1 1 1] Do we have the means to open the door?
    (if (`self.CanOpen`)
      ;[1 1 1] Unlock the door
      (set `self.Locked` false)
      (`PrimitiveComponent.SetMaterial` (`self.Door_Small_UI`) 0 "/Game/ModSci_Engineer/Materials/UI/MI_Door_Unlocked.MI_Door_Unlocked")
      (`LightComponent.SetLightColor` (`self.PointLightb`) (`self.UnlockedLightColor`) true)
      (`LightComponent.SetLightColor` (`self.PointLight`) (`self.UnlockedLightColor`) true)
      (`AudioComponent.Play` _unlockdoor 0.0)
      (`KismetSystemLibrary.Delay` (+ (`SoundBase.Duration` (`AudioComponent.Sound` _unlockdoor)) 0.7))
      ;[1 1 1] Try to open the door
      (if (`self.Interactable`) :!label _label_2
        ;[1 1 1] Play sound, particles
        (`AudioComponent.Play` (`self.DoorSwish`) 0.0)
        (`ActorComponent.Activate` (`self.SteamDoor`) false)
        (`ActorComponent.Activate` (`self.SteamDoor2`) false)
        (set `self.Interactable` false)
        (goto _label))
      (else
        ;[1 1 1] If this door can be unlocked, let the player know how to unlock it
        (if (> (`self.KeyID`) -1)
          (bind _asbp_player_controller (cast `/Game/Haywire/Blueprints/Player/BP_PlayerController` (`GameplayStatics.GetPlayerController` 0)))
          (`/Game/Haywire/Blueprints/Player/BP_PlayerController.Play Message` _asbp_player_controller "NewEnumerator0" 2.0 (`self.KeyID`) ""))))
    (else
      (goto _label_2))))

(event `self.Trigger.OnComponentEndOverlap`
  (params (OverlappedComponent :type "PrimitiveComponent Object Reference") (OtherActor :type "Actor Object Reference") (OtherComp :type "PrimitiveComponent Object Reference") (OtherBodyIndex :type Integer))
  ;[1 1 1] Begin closing door
  (set `self.InTrigger` false)
  (if (not (`self.Interactable`))
    (`TimelineComponent.Stop` (`self.Timeline_0`))
    (`AudioComponent.Play` (`self.DoorSwish`) 0.0)
    (goto _label :!via `Reverse`)))

(event `self.Trigger.OnComponentBeginOverlap`
  (params (OverlappedComponent :type "PrimitiveComponent Object Reference") (OtherActor :type "Actor Object Reference") (OtherComp :type "PrimitiveComponent Object Reference") (OtherBodyIndex :type Integer) (bFromSweep :type Boolean) (SweepResult :type "HitResult Structure (by ref)"))
  (set `self.InTrigger` true))

(fn `CanOpen`
  (returns (`Open?` :type Boolean))
  (if (`self.Locked`)
    (bind _asbp_player_controller (cast `/Game/Haywire/Blueprints/Player/BP_PlayerController` (`GameplayStatics.GetPlayerController` 0)))
    (if (`/Game/Haywire/Blueprints/Player/BP_PlayerController.HasKey` _asbp_player_controller (`self.KeyID`))
      (return true)
      (else
        (return false)))
    (else
      (return true))))

(fn `UserConstructionScript`
  (bind _door_small_ui (`self.Door_Small_UI`))
  (if (`self.Locked`)
    (`PrimitiveComponent.SetMaterial` _door_small_ui 0 "/Game/ModSciInteriors/Materials/UI/MI_Door_Locked.MI_Door_Locked")
    (`LightComponent.SetLightColor` (`self.PointLight`) (`self.LockedLightColor`) true)
    (`LightComponent.SetLightColor` (`self.PointLightb`) (`self.LockedLightColor`) true)
    (else
      (`PrimitiveComponent.SetMaterial` _door_small_ui 0 "/Game/ModSciInteriors/Materials/UI/MI_Door_Unlocked.MI_Door_Unlocked")
      (`LightComponent.SetLightColor` (`self.PointLightb`) (`self.UnlockedLightColor`) true)
      (`LightComponent.SetLightColor` (`self.PointLight`) (`self.UnlockedLightColor`) true))))