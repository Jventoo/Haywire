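; BP_BigDoor is a large door actor that opens by sliding down and closes by rising back up.
; On BeginPlay it treats its placed location as open or closed based on IsOpen, then derives the other position by offsetting Z by DoorSize.
; OpenDoor and CloseDoor events play a timeline forward or in reverse, lerping the whole actor between the two positions without sweep.
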(event `self.ReceiveBeginPlay`
  (if (`self.IsOpen`)
    (bind _output_get (set `self.OpenDoorPos` (`self.K2_GetActorLocation`)))
    (set `self.ClosedDoorPos` (`KismetMathLibrary.MakeVector` (.x _output_get) (.y _output_get) (+ (.z _output_get) (`self.DoorSize`))))
    (else
      (bind _output_get_2 (set `self.ClosedDoorPos` (`self.K2_GetActorLocation`)))
      (set `self.OpenDoorPos` (`KismetMathLibrary.MakeVector` (.x _output_get_2) (.y _output_get_2) (- (.z _output_get_2) (`self.DoorSize`)))))))

(event `OpenDoor`
  (bind (_direction _doorpos) (`Timeline|DoorTimeline` :!via `PlayFromStart` :!label _label)
    (:`Update`
      (`self.K2_SetActorLocation` (`KismetMathLibrary.VLerp` (`self.ClosedDoorPos`) (`self.OpenDoorPos`) _doorpos)))))

(event `CloseDoor`
  (goto _label :!via `ReverseFromEnd`))

(fn `UserConstructionScript`)