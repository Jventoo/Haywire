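; BP_DoorControl is an interactable that triggers a one-time scripted door and audio sequence.
; On first Interact, it plays tension music at its location, calls CloseDoor on the RaiseDoors list and OpenDoor on the LowerDoors list.
; After timed delays it spawns chase audio attached to the player character's mesh, then destroys the referenced ShieldActor.
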(event `/Game/Haywire/Blueprints/Interactions/BPI_Interaction.Interact`
  (`/Engine/EditorBlueprintResources/StandardMacros.DoOnce` false
    (:`Completed`
      (`GameplayStatics.PlaySoundAtLocation` "/Game/Haywire/Audio/Music/SC_TensionMusic.SC_TensionMusic" (`self.K2_GetActorLocation`) (struct) 1.0 1.0 4.0 null null null)
      (for _array_element (`self.RaiseDoors`)
        (`/Game/Haywire/Blueprints/Interactions/Doors/BP_BigDoor.CloseDoor` _array_element))
      (for _array_element_2 (`self.LowerDoors`)
        (`/Game/Haywire/Blueprints/Interactions/Doors/BP_BigDoor.OpenDoor` _array_element_2))
      (`KismetSystemLibrary.Delay` 8.0)
      (`GameplayStatics.SpawnSoundAttached` "/Game/Haywire/Audio/Music/SC_Chase.SC_Chase" (`Character.Mesh` (`GameplayStatics.GetPlayerCharacter` 0)) "None" (-800.0 0.0 0.0) (struct) "KeepRelativeOffset" false 1.0 1.0 0.0 null null)
      (`KismetSystemLibrary.Delay` 2.0)
      (`self.K2_DestroyActor` (`self.ShieldActor`)))))

(fn `UserConstructionScript`)