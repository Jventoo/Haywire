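; Trigger volume that streams Haywire levels in and out as the player passes through, doubling as a save checkpoint.
; On player overlap it block-loads the game mode's next level, records the player's location, increments the saved current level and writes the save slot.
; When the player leaves, it asynchronously unloads the level returned by the game mode's GetCurrentLevel.
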(event `self.Box.OnComponentBeginOverlap`
  (params (OverlappedComponent :type "PrimitiveComponent Object Reference") (OtherActor :type "Actor Object Reference") (OtherComp :type "PrimitiveComponent Object Reference") (OtherBodyIndex :type Integer) (bFromSweep :type Boolean) (SweepResult :type "HitResult Structure (by ref)"))
  (bind _returnvalue (`GameplayStatics.GetPlayerCharacter` 0))
  (if (== OtherActor _returnvalue)
    (bind _ashaywire_gm (cast `/Game/Haywire/Blueprints/Game/HaywireGM` (`GameplayStatics.GetGameMode`)))
    (`GameplayStatics.LoadStreamLevel` (`/Game/Haywire/Blueprints/Game/HaywireGM.GetNextLevel` _ashaywire_gm) true true)
    (bind _savegameref (`/Game/Haywire/Blueprints/Game/HaywireGM.SaveGameRef` _ashaywire_gm))
    (set `/Game/Haywire/Blueprints/Game/BP_SaveGame.PlayerLocation` (`self.K2_GetActorLocation` _returnvalue) _savegameref)
    (set `/Game/Haywire/Blueprints/Game/BP_SaveGame.CurrentLevel` (+ (`/Game/Haywire/Blueprints/Game/BP_SaveGame.CurrentLevel` _savegameref) 1) _savegameref)
    (`GameplayStatics.SaveGameToSlot` _savegameref (`/Game/Haywire/Blueprints/Game/HaywireGM.SaveGameSlot` _ashaywire_gm))))

(event `self.Box.OnComponentEndOverlap`
  (params (OverlappedComponent :type "PrimitiveComponent Object Reference") (OtherActor :type "Actor Object Reference") (OtherComp :type "PrimitiveComponent Object Reference") (OtherBodyIndex :type Integer))
  (if (== OtherActor (`GameplayStatics.GetPlayerCharacter` 0))
    (bind _ashaywire_gm (cast `/Game/Haywire/Blueprints/Game/HaywireGM` (`GameplayStatics.GetGameMode`)))
    (`GameplayStatics.UnloadStreamLevel` (`/Game/Haywire/Blueprints/Game/HaywireGM.GetCurrentLevel` _ashaywire_gm))))

(fn `UserConstructionScript`)