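; Player controller for Haywire that handles pausing and tracks the keys the player has collected.
; The Pause input toggles a WB_PauseMenu widget, switching game pause, mouse cursor and input mode along with it.
; AddKey and HasKey store and check key IDs in a Keys collection.
; PlayMessage creates a widget, but no class is set and the message is not used.
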(event `InputAction|Pause` :paused true
  (params (Key :type "Key Structure"))
  (:`Pressed`
    (if (`self.PauseOpen`)
      (`self.UnPauseGame`)
      (else
        (`self.PauseGame`)))))

(fn `AddKey`
  (params (KeyID :type Integer))
  (`BlueprintSetLibrary.Set_Add` (`self.Keys`) KeyID))

(fn `HasKey`
  (params (KeyID :type Integer))
  (returns (Bool :type Boolean))
  (return (`BlueprintSetLibrary.Set_Contains` (`self.Keys`) KeyID)))

(fn `PauseGame`
  (set `self.PauseOpen` true)
  (bind _returnvalue (`|CreateWidget` "/Game/Haywire/Blueprints/UI/MainMenu/WB_PauseMenu.WB_PauseMenu_C" self))
  (bind _output_get (set `self.PauseRef` _returnvalue))
  (`UserWidget.AddToViewport` _returnvalue 0)
  (`UserWidget.AddToViewport` _output_get 0)
  (set `self.bShowMouseCursor` true)
  (`WidgetBlueprintLibrary.SetInputMode_GameAndUIEx` self _output_get)
  (`GameplayStatics.SetGamePaused` true))

(fn `PlayMessage`
  (params (Message :type "/Game/Haywire/Blueprints/UI/HUD/MessageType Enum" :default "NewEnumerator0"))
  (`|CreateWidget` null))

(fn `UnPauseGame`
  (bind _pauseref (`self.PauseRef`))
  (set `self.PauseOpen` false)
  (`/Engine/EditorBlueprintResources/StandardMacros.IsValid` _pauseref
    (:`Is Valid`
      (`Widget.RemoveFromParent` _pauseref))
    (:`Is Not Valid`
      _))
  (set `self.bShowMouseCursor` false)
  (`WidgetBlueprintLibrary.SetInputMode_GameOnly` self)
  (`GameplayStatics.SetGamePaused` false))

(fn `UserConstructionScript`)