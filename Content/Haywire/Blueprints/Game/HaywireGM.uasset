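; Haywire game mode that sets up the player's save game at BeginPlay and supplies level names derived from saved progress.
; An existing BP_SaveGame is loaded and the player character is teleported to its saved location.
; Otherwise a new save records the character's current location and is written asynchronously.
; GetCurrentLevel and GetNextLevel format "Level{ID}" names from the saved CurrentLevel and the number after it.
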(event `self.ReceiveBeginPlay`
  (bind _returnvalue (`GameplayStatics.DoesSaveGameExist` (`self.SaveGameSlot`)))
  (if _returnvalue
    (bind _returnvalue_2 (`GameplayStatics.LoadGameFromSlot` (`self.SaveGameSlot`)))
    (bind _asbp_save_game (cast `/Game/Haywire/Blueprints/Game/BP_SaveGame` _returnvalue_2))
    (set `self.SaveGameRef` _asbp_save_game)
    (`self.K2_SetActorLocation` (`GameplayStatics.GetPlayerCharacter` 0) (`/Game/Haywire/Blueprints/Game/BP_SaveGame.PlayerLocation` _asbp_save_game) false true)
    (else
      (bind _returnvalue_3 (`GameplayStatics.CreateSaveGameObject` "/Game/Haywire/Blueprints/Game/BP_SaveGame.BP_SaveGame_C"))
      (bind _output_get (set `self.SaveGameRef` _returnvalue_3))
      (set `/Game/Haywire/Blueprints/Game/BP_SaveGame.PlayerLocation` (`self.K2_GetActorLocation` (`GameplayStatics.GetPlayerCharacter` 0)) _returnvalue_3)
      (`AsyncActionHandleSaveGame.AsyncSaveGameToSlot` _output_get (`self.SaveGameSlot`)))))

(fn `GetCurrentLevel`
  (returns (Level :type Name))
  (return (`KismetStringLibrary.Conv_StringToName` (`KismetSystemLibrary.MakeLiteralString` (`KismetTextLibrary.Conv_TextToString` (`|FormatText` "Level{ID}" (`/Game/Haywire/Blueprints/Game/BP_SaveGame.CurrentLevel` (`self.SaveGameRef`))))))))

(fn `GetNextLevel`
  (returns (Level :type Name))
  (return (`KismetStringLibrary.Conv_StringToName` (`KismetSystemLibrary.MakeLiteralString` (`KismetTextLibrary.Conv_TextToString` (`|FormatText` "Level{ID}" (+ (`/Game/Haywire/Blueprints/Game/BP_SaveGame.CurrentLevel` (`self.SaveGameRef`)) 1)))))))

(fn `UserConstructionScript`)